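; Geolocation system for the Speedup game that manages device location services and reports path distance and speed for NFT items to the server.
; It initializes location services on BeginPlay, polls their status on a timer, and ReInitServis retries with fallback accuracy before starting them.
; Helpers supply last location and point-to-point distance, while path events send updates through the GameMode's HTTPAPI.
; Per-slot tracking timers call TickEvent01, whose aggregation logic is disconnected.
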(event Custom|CheckGeodataCheck
  (bind _returnvalue (Class|LocationServices|AreLocationServicesEnabled))
  (Class|SpeedupGeoDataSystem|SetServiceEnable _returnvalue)
  (Development|PrintString (Utilities|String|Append "Service location - " (Utilities|String|ToString(Boolean) (Variables|Default|GetServiceEnable))) true true "(R=0.052660,G=0.338542,B=0.048083,A=1.000000)" 6.0))

(event Custom|TryStartService
  (Utilities|FlowControl|Delay 1.0)
  (bind _returnvalue (Class|LocationServices|StartLocationServices))
  (Class|SpeedupGeoDataSystem|SetServiceStart _returnvalue)
  (Development|PrintString (Utilities|String|Append "Service was START - " (Utilities|String|ToString(Boolean) _returnvalue)) true true "(R=0.000000,G=0.796875,B=0.270036,A=1.000000)" 4.0))

(event Custom|SendPartPath_Event_0
  (params (Path :type Integer))
  (bind _activpath (Variables|Default|GetActivPath))
  (bind _output (Utilities|Array|Get(acopy) _activpath Path))
  (bind _partsofpath (Variables|/Script/speedup.GeoPath|GetPartsOfPath _output))
  (bind _returnvalue (Utilities|Array|LastIndex _partsofpath))
  (bind _output_2 (Utilities|Array|Get(acopy) _partsofpath _returnvalue))
  (bind (_pathid _itemid _slotid _pathlength _pathtime _minspeed _maxspeed _averagespeed) (Utilities|Struct|BreakGeoPathinfo _output_2))
  (bind _asmouse_game_mode (Utilities|Casting|CastToMouse_GameMode (Game|GetGameMode)))
  (Class|HTTPAPIComponent|NFTUpdateRequest (Variables|/Game/Speedup/Blueprints/Mouse_GameMode.Mouse_GameMode_C|GetHTTPAPI _asmouse_game_mode) _itemid _pathid _pathlength _averagespeed)
  (Development|PrintString (Utilities|String|ToString(Text) (Utilities|Text|FormatText "NFT Update Request 
Distance - {Dist} 
Speed - {Speed}" (Utilities|Text|ToText(Float) _pathlength "HalfToEven" false true 4 324 4 4) (Utilities|Text|ToText(Float) _averagespeed "HalfToEven" false true 4 324 4 4)))))

(event Custom|CustomEvent_03
  (CallFunction|TickEvent01 2))

(event Custom|CustomEvent_01
  (CallFunction|TickEvent01))

(event Custom|CustomEvent_02
  (CallFunction|TickEvent01 1))

(event EventBeginPlay
  (Utilities|Time|SetTimerbyEvent (delegate Custom|CheckGeodataCheck) 8.0 true)
  (bind _returnvalue (Class|LocationServices|AreLocationServicesEnabled))
  (Class|SpeedupGeoDataSystem|SetServiceEnable _returnvalue)
  (if _returnvalue
    (bind _returnvalue_2 (Class|LocationServices|InitLocationServices "LA_Best" 1e+03 1e+01))
    (Class|SpeedupGeoDataSystem|SetServiceInit _returnvalue_2)
    (else
      (Class|SpeedupGeoDataSystem|SetServiceInit false)
      (Class|SpeedupGeoDataSystem|SetServiceStart false)
      (Variables|Default|SetErrorText "Service dont enable"))))

(event EventTick
  (params (DeltaSeconds :type Float%20%28single-precision%29)))

(event EventUpdateLocation)

(event EventStartTrackPathEvent
  (params (Stop :type Boolean) (ItemID :type Integer) (PathID :type Integer) (SlotID :type Integer))
  (if (not Stop)
    (switch int SlotID
      (:0
        (Utilities|Time|SetTimerbyEvent (delegate Custom|CustomEvent_01) 2.0 true))
      (:1
        (Utilities|Time|SetTimerbyEvent (delegate Custom|CustomEvent_02) 2.0 true))
      (:2
        (Utilities|Time|SetTimerbyEvent (delegate Custom|CustomEvent_03) 2.0 true)))))

(fn GetLastLocation
  (bind _returnvalue (Class|LocationServices|GetLastKnownLocation))
  (bind _output_get (Variables|Default|SetTimestamp (.Timestamp (Utilities|Struct|BreakLocationServicesData _returnvalue))))
  (Development|PrintString (Utilities|String|ToString(Text) (Utilities|Text|FormatText "Function - get last location 
Longitude - {Lon} 
Latitude - {Lat}" (Utilities|Text|ToText(Float) (.Longitude (Utilities|Struct|BreakLocationServicesData _returnvalue)) "HalfToEven" false true 4 324 4) (Utilities|Text|ToText(Float) (.Latitude (Utilities|Struct|BreakLocationServicesData _returnvalue)) "HalfToEven" false true 4 324 4))) true true "(R=0.074954,G=0.000000,B=0.265625,A=1.000000)" 4.0)
  (return (Utilities|Struct|MakeGeoLocationInfo (Math|Vector2D|MakeVector2D (.Longitude (Utilities|Struct|BreakLocationServicesData _returnvalue)) (.Latitude (Utilities|Struct|BreakLocationServicesData _returnvalue))) _output_get)))

(fn GetDistanse2Coor
  (params (PointStart :type Geo%20Point%20Info%20Structure) (PointEnd :type Geo%20Point%20Info%20Structure))
  (bind _pointlocation (Utilities|Struct|BreakGeoPointInfo PointStart))
  (bind _pointlocation_2 (Utilities|Struct|BreakGeoPointInfo PointEnd))
  (bind (_x _y) (Math|Vector2D|BreakVector2D _pointlocation))
  (bind (_x_2 _y_2) (Math|Vector2D|BreakVector2D _pointlocation_2))
  (|CallParentFunction PointStart PointEnd)
  (bind _returnvalue (Class|GeoLocationUtilities|CalculateDistanceBetween (Utilities|Struct|MakeGeoCoordinate _x _y) (Utilities|Struct|MakeGeoCoordinate _x_2 _y_2)))
  (Development|PrintText (Utilities|Text|FormatText "Distance is {D}" (Utilities|Text|ToText(Float) (Math|Float|Absolute(Float) _returnvalue) "HalfToEven" false true 4 324 4 4)))
  (return (Math|Float|Absolute(Float) _returnvalue)))

(fn ReInitServis
  (Development|PrintText "Start ReInit GEOLOCATION serves" true true "(R=0.071648,G=0.239583,B=0.000000,A=1.000000)")
  (bind _returnvalue (Class|LocationServices|AreLocationServicesEnabled))
  (Class|SpeedupGeoDataSystem|SetServiceEnable _returnvalue)
  (Development|PrintText (Utilities|Text|FormatText "GEOLOCATION serves enable is - {Result}" _returnvalue) true true "(R=0.071648,G=0.239583,B=0.000000,A=1.000000)")
  (if _returnvalue
    (Development|PrintText "Service is enable" true true "(R=0.236779,G=0.849000,B=0.000000,A=1.000000)" 1e+01)
    (bind _returnvalue_2 (Class|LocationServices|IsLocationAccuracyAvailable "LA_Best"))
    (if _returnvalue_2
      (bind _returnvalue_3 (Class|LocationServices|InitLocationServices "LA_Best" 1e+03 1e+01))
      (Class|SpeedupGeoDataSystem|SetServiceInit _returnvalue_3)
      (if (Variables|Default|GetServiceInit)
        (Development|PrintText "Init Geolocation servis " true true "(R=0.409894,G=0.849000,B=0.000000,A=1.000000)" 1e+01)
        (bind _output_get (Variables|Default|SetErrorText "Success"))
        (Development|PrintText (Utilities|Text|FormatText "Init location Servis Best is {Result}" _output_get) true true "(R=0.071648,G=0.239583,B=0.000000,A=1.000000)")
        (CallFunction|TryStartService)
        (else
          (Development|PrintText "werror in init Servis Best " true true "(R=0.849000,G=0.023099,B=0.000000,A=1.000000)" 1e+01)
          (Variables|Default|SetErrorText "Service dont enable")))
      (else
        (Development|PrintText "Geolocation Best is't aviable" true true "(R=0.849000,G=0.023099,B=0.000000,A=1.000000)" 1e+01)
        (bind _returnvalue_4 (Class|LocationServices|IsLocationAccuracyAvailable "LA_TenMeters"))
        (if _returnvalue_4
          (bind _returnvalue_5 (Class|LocationServices|InitLocationServices "LA_OneKilometer" 1e+02 2.0))
          (Class|SpeedupGeoDataSystem|SetServiceInit _returnvalue_5)
          (if (Variables|Default|GetServiceInit)
            (Variables|Default|SetErrorText "Success")
            (CallFunction|TryStartService)
            (else
              (Variables|Default|SetErrorText "Service don't enable")))
          (else
            (Development|PrintText "Geolocation is't aviable" true true "(R=0.849000,G=0.023099,B=0.000000,A=1.000000)" 1e+01)
            (Class|SpeedupGeoDataSystem|SetServiceInit false)
            (Variables|Default|SetErrorText "Service don't aviable")))))
    (else
      (Class|SpeedupGeoDataSystem|SetServiceInit false)
      (Class|SpeedupGeoDataSystem|SetServiceStart false)
      (Variables|Default|SetErrorText "Service dont enable")
      (Development|PrintText "Service dont enable" true true "(R=0.849000,G=0.023099,B=0.000000,A=1.000000)" 1e+01)
      (Math|Integer|IncrementInt (Variables|Default|GetCount)
        (:%20%20
          (Variables|Default|SetCount (Variables|Default|GetCount))
          (if (> (Variables|Default|GetCount) 10)
            (bind _asmouse_game_mode (Utilities|Casting|CastToMouse_GameMode (Game|GetGameMode)))
            (Class|SpeedupGameModeBase|AddPopAppMessage _asmouse_game_mode "" "P" "error")))))))

(fn TickEvent01
  (params (SlotN :type Integer)))

(fn UpdateDistance
  (params (DeactivePathID :type Integer) (DeactivNFDId :type Integer) (avg_velocity :type Float%20%28single-precision%29) (avg_distance :type Float%20%28single-precision%29))
  (if (Variables|Default|GetServiceInit)
    _
    (else
      (CallFunction|ReInitServis)))
  (bind _asmouse_game_mode (Utilities|Casting|CastToMouse_GameMode (Game|GetGameMode)))
  (Class|HTTPAPIComponent|NFTUpdateRequest (Variables|/Game/Speedup/Blueprints/Mouse_GameMode.Mouse_GameMode_C|GetHTTPAPI _asmouse_game_mode) DeactivNFDId DeactivePathID avg_velocity avg_distance)
  (Development|PrintString (Utilities|String|ToString(Text) (Utilities|Text|FormatText "Function - UpdateDistunce 
Longitude - {Lon} 
Latitude - {Lat} 
PathID - {Path}" (Utilities|Text|ToText(Float) avg_velocity "HalfToEven" false true 4 324 4) (Utilities|Text|ToText(Float) avg_distance "HalfToEven" false true 4 324 4) DeactivePathID)) true true "(R=0.074954,G=0.000000,B=0.265625,A=1.000000)" 4.0))