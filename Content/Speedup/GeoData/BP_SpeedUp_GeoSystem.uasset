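; Geolocation system Blueprint that wraps device location services and reports path stats to the NFT update API.
; BeginPlay initializes location services; a separate event starts them and stores location changes.
; Overrides supply last known location and coordinate distance, while SendPartPath and UpdateDistance send stats through Mouse_GameMode's HTTPAPI.
; Slot timers call TickEvent01 every two seconds, but its path-aggregation logic is disconnected, so it does nothing.
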(event Custom|StarServiceInBP
  (if (Variables|Default|GetServiceInit)
    (bind _returnvalue (Class|LocationServices|StartLocationServices))
    (if _returnvalue
      (Variables|Default|SetErrorText "No")
      (Variables|Default|SetReady true)
      (bind _returnvalue_2 (Class|LocationServices|GetLocationServicesImpl))
      (EventDispatchers|AssignOnLocationChanged _returnvalue_2 (delegate Custom|OnLocationChanged_Event_0))
      (else
        (Variables|Default|SetErrorText "Service dont Start")))
    (else
      (Class|SpeedupGeoDataSystem|SetServiceStart false)
      (Variables|Default|SetErrorText "Service dont Init"))))

(event Custom|OnLocationChanged_Event_0
  (params (LocationData :type Location%20Services%20Data%20Structure))
  (bind _output_get (Variables|Default|SetLocation%20DataFronEvent LocationData))
  (Variables|Default|SetPointFromServis (Utilities|Struct|MakeGeoPointInfo 0 (Math|Vector2D|MakeVector2D (.Timestamp (Utilities|Struct|BreakLocationServicesData _output_get)) (.Longitude (Utilities|Struct|BreakLocationServicesData _output_get))) 0.0 0.0 0.0 "0001.01.01-00.00.00" "0001.01.01-00.00.00" "Path")))

(event Custom|SendPartPath_Event_0
  (params (Path :type Integer))
  (bind _activpath (Variables|Default|GetActivPath))
  (bind _output (Utilities|Array|Get(acopy) _activpath Path))
  (bind _partsofpath (Variables|/Script/speedup.GeoPath|GetPartsOfPath _output))
  (bind _returnvalue (Utilities|Array|LastIndex _partsofpath))
  (bind _output_2 (Utilities|Array|Get(acopy) _partsofpath _returnvalue))
  (bind (_pathid _itemid _slotid _pathlength _pathtime _minspeed _maxspeed _averagespeed) (Utilities|Struct|BreakGeoPathinfo _output_2))
  (bind _asmouse_game_mode (Utilities|Casting|CastToMouse_GameMode (Game|GetGameMode)))
  (Class|HTTPAPIComponent|NFTUpdateRequest (Variables|/Game/Speedup/Blueprints/Mouse_GameMode.Mouse_GameMode_C|GetHTTPAPI _asmouse_game_mode) _itemid _pathid _pathlength _averagespeed)
  (Development|PrintString "NFT Update Request"))

(event Custom|CustomEvent_03
  (CallFunction|TickEvent01 1))

(event Custom|CustomEvent_01
  (CallFunction|TickEvent01))

(event Custom|CustomEvent_02
  (CallFunction|TickEvent01 1))

(event EventBeginPlay
  (EventDispatchers|AssignSendPartPath self (delegate Custom|SendPartPath_Event_0))
  (bind _returnvalue (Class|LocationServices|AreLocationServicesEnabled))
  (Class|SpeedupGeoDataSystem|SetServiceEnable _returnvalue)
  (if _returnvalue
    (bind _returnvalue_2 (Class|LocationServices|InitLocationServices "LA_Best" 1e+03 1e+01))
    (Class|SpeedupGeoDataSystem|SetServiceInit _returnvalue_2)
    (else
      (Class|SpeedupGeoDataSystem|SetServiceInit false)
      (Class|SpeedupGeoDataSystem|SetServiceStart false)
      (Variables|Default|SetErrorText "Service dont enable"))))

(event EventTick
  (params (DeltaSeconds :type Float%20%28single-precision%29)))

(event EventUpdateLocation)

(event EventStartTrackPathEvent
  (params (Stop :type Boolean) (ItemID :type Integer) (PathID :type Integer) (SlotID :type Integer))
  (if (not Stop)
    (switch int SlotID
      (:0
        (Utilities|Time|SetTimerbyEvent (delegate Custom|CustomEvent_01) 2.0 true))
      (:1
        (Utilities|Time|SetTimerbyEvent (delegate Custom|CustomEvent_02) 2.0 true))
      (:2
        (Utilities|Time|SetTimerbyEvent (delegate Custom|CustomEvent_03) 2.0 true)))))

(fn GetLastLocation
  (bind _returnvalue (Class|LocationServices|GetLastKnownLocation))
  (bind _output_get (Variables|Default|SetTimestamp (.Timestamp (Utilities|Struct|BreakLocationServicesData _returnvalue))))
  (return (Utilities|Struct|MakeGeoLocationInfo (Math|Vector2D|MakeVector2D (.Longitude (Utilities|Struct|BreakLocationServicesData _returnvalue)) (.Latitude (Utilities|Struct|BreakLocationServicesData _returnvalue))) _output_get)))

(fn GetDistanse2Coor
  (params (PointStart :type Geo%20Point%20Info%20Structure) (PointEnd :type Geo%20Point%20Info%20Structure))
  (bind _pointlocation (Utilities|Struct|BreakGeoPointInfo PointStart))
  (bind _pointlocation_2 (Utilities|Struct|BreakGeoPointInfo PointEnd))
  (bind (_x _y) (Math|Vector2D|BreakVector2D _pointlocation))
  (bind (_x_2 _y_2) (Math|Vector2D|BreakVector2D _pointlocation_2))
  (|CallParentFunction PointStart PointEnd)
  (bind _returnvalue (Class|GeoLocationUtilities|CalculateDistanceBetween (Utilities|Struct|MakeGeoCoordinate _x _y) (Utilities|Struct|MakeGeoCoordinate _x_2 _y_2)))
  (return (Math|Float|Absolute(Float) _returnvalue)))

(fn ReInitServis
  (bind _returnvalue (Class|LocationServices|AreLocationServicesEnabled))
  (Class|SpeedupGeoDataSystem|SetServiceEnable _returnvalue)
  (if true
    (bind _returnvalue_2 (Class|LocationServices|InitLocationServices "LA_Best" 1e+02 2.0))
    (Class|SpeedupGeoDataSystem|SetServiceInit _returnvalue_2)
    (Class|LocationServices|StartLocationServices)
    (else
      (Class|SpeedupGeoDataSystem|SetServiceInit false)
      (Class|SpeedupGeoDataSystem|SetServiceStart false)
      (Variables|Default|SetErrorText "Service dont enable"))))

(fn TickEvent01
  (params (SlotN :type Integer)))

(fn UpdateDistance
  (params (DeactivePathID :type Integer) (DeactivNFDId :type Integer) (avg_velocity :type Integer) (avg_distance :type Integer))
  (bind _asmouse_game_mode (Utilities|Casting|CastToMouse_GameMode (Game|GetGameMode)))
  (Class|HTTPAPIComponent|NFTUpdateRequest (Variables|/Game/Speedup/Blueprints/Mouse_GameMode.Mouse_GameMode_C|GetHTTPAPI _asmouse_game_mode) DeactivNFDId DeactivePathID (Math|Conversions|ToFloat(Integer) avg_velocity) (Math|Conversions|ToFloat(Integer) avg_distance)))