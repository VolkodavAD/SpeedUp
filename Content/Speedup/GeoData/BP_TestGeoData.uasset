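; BP_TestGeoData is a test Blueprint for saving geo path data to a DataTable.
; SavePath constructs a BP_GeoPath, fills it with a hardcoded velocity range and sample points, then saves it under an incremented ID as row name.
; Nothing in the file runs this: the events are empty, the SavePath call is disconnected, and GetLastPosition returns immediately.
; Unreachable leftover nodes sketch reading rows back from the table.
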(event Custom|CheckLaspPositiom)

(event EventBeginPlay)

(event Collision|EventActorBeginOverlap
  (params (OtherActor :type Actor%20Object%20Reference)))

(event EventTick
  (params (DeltaSeconds :type Float%20%28single-precision%29)))

(event EventDestroyed)

(event EventEndPlay
  (params (EndPlayReason :type EEndPlayReason%20Enum :default "Destroyed")))

(fn ConstructionScript)

(fn GetLastPosition
  (return ""))

(fn SavePath
  (bind _returnvalue (Game|ConstructObjectfromClass "/Game/Speedup/GeoData/BP_GeoPath.BP_GeoPath_C"))
  (bind _output_get (Variables|Default|SetGeoPuth _returnvalue))
  (Utilities|IsValid _output_get
    (:Is%20Valid
      (Variables|/Script/speedup.GeoPath|SetPlayerPathInfo _output_get (Utilities|Struct|MakeGeoPathinfo 0 0.0 0 1.0 5.0 (Utilities|Array|MakeArray (Utilities|Struct|MakeGeoPointInfo 0 "(X=0.000000,Y=0.000000)" 0.0 "0001.01.01-00.00.00" "point1") (Utilities|Struct|MakeGeoPointInfo 0 "(X=5.000000,Y=5.000000)" 0.0 "0001.01.01-00.00.00" "point2" "(X=5.000000,Y=5.000000)") (Utilities|Struct|MakeGeoPointInfo 0 "(X=10.000000,Y=10.000000)" 0.0 "0001.01.01-00.00.00" "point3" "(X=10.000000,Y=10.000000)"))))
      (bind _result (Math|Integer|IncrementInt (Variables|Default|GetID))
        (:%20%20
          (bind _output_get_2 (Variables|Default|SetID _result))
          (bind _returnvalue_2 (Class|GeoPath|SavePuthinDataTable (Variables|Default|GetGeoPuth) (Utilities|String|ToString(Integer) _output_get_2) (Variables|Default|GetData%20Table%20Puths)))
          (return _returnvalue_2))))))