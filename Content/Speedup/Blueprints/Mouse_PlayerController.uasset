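; Player controller that detects touch swipes by comparing press and release screen positions.
; On release it runs vertical and horizontal checks with a fixed pixel threshold, setting flags that are never cleared here.
; Vertical detection covers only downward drags, while a leftward drag sets HorizontalSwipeRight and a rightward one HorizontalSwipeLeft.
; The scroll-priority check is reachable only from disconnected debug nodes.
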(event EventBeginPlay)

(event EventTick
  (params (DeltaSeconds :type Float%20%28single-precision%29)))

(event Input|TouchEvents|InputTouch
  (params (Location :type Vector) (FingerIndex :type ETouchIndex%20Enum))
  (bind (_x _y) (Math|Vector|BreakVector Location))
  (:Pressed
    (Variables|Default|SetisPressed true)
    (Variables|Default|SetvectorStart (Math|Vector2D|MakeVector2D _x _y)))
  (:Released
    (Variables|Default|SetvectorStop (Math|Vector2D|MakeVector2D _x _y))
    (Utilities|FlowControl|Sequence
      (:then_0
        (CallFunction|CheckVerticalSwipe))
      (:then_1
        (CallFunction|CheckHorizontalSwipe)))))

(fn ConstructionScript)

(fn CheckVerticalSwipe
  (if (< (- (.Y (Math|Vector2D|BreakVector2D (Variables|Default|GetvectorStart))) (.Y (Math|Vector2D|BreakVector2D (Variables|Default|GetvectorStop)))) -1e+02)
    (Variables|Default|SetVerticalSwipe true)))

(fn CheckHorizontalSwipe
  (bind _vectorstart (Variables|Default|GetvectorStart))
  (bind _vectorstop (Variables|Default|GetvectorStop))
  (bind _x (Math|Vector2D|BreakVector2D _vectorstart))
  (bind _x_2 (Math|Vector2D|BreakVector2D _vectorstop))
  (bind _returnvalue (- _x _x_2))
  (if (> _returnvalue 1e+02)
    (Variables|Default|SetHorizontalSwipeRight true)
    (elif (< _returnvalue -1e+02)
      (Variables|Default|SetHorizontalSwipeLeft true))))

(fn CheckScrollInput
  (bind _vectorstart (Variables|Default|GetvectorStart))
  (bind (_x _y) (Math|Vector2D|BreakVector2D _vectorstart))
  (if (< _x _y)
    (Variables|Default|SetScrollPriority true)
    (Development|PrintString "scroll priority true" true true "(R=1.000000,G=0.040100,B=0.000000,A=1.000000)" 5.0)
    (else
      (Variables|Default|SetScrollPriority false))))