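; Game instance that exposes sign-in state, logout and widget helpers for the Speedup game.
; Sign-in helpers read or set SignedIn on BP_LoginGameMode, so they act only when that game mode is active.
; Logout requests MapLogin, then, if the current game mode and HUD are the login ones, clears SignedIn and shows the sign-in widget.
; M_AddWidget forwards to WidgetManager, while GetWidget is an empty stub.
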(fn GetWidget
  (params (name :type String)))

(fn Logout
  (Game|OpenLevel(byName) "MapLogin")
  (bind _asbp_login_game_mode (Utilities|Casting|CastToBP_LoginGameMode (Game|GetGameMode)))
  (bind _output_get (Variables|Default|SetAs%20BP%20Login%20Game%20Mode _asbp_login_game_mode))
  (bind _asbp_login_hud (Utilities|Casting|CastToBP_LoginHUD (HUD|GetHUD (Game|GetPlayerController 0))))
  (Variables|Default|SetAs%20BP%20Login%20HUD _asbp_login_hud)
  (Variables|/Game/Speedup/Blueprints/BP_LoginGameMode.BP_LoginGameMode_C|SetSignedIn _output_get false)
  (Default|Logout (Variables|Default|GetAs%20BP%20Login%20HUD))
  (Default|MovetoSigninWidget (Variables|Default|GetAs%20BP%20Login%20HUD)))

(fn SignedinTrue
  (bind _asbp_login_game_mode (Utilities|Casting|CastToBP_LoginGameMode (Game|GetGameMode)))
  (bind _output_get (Variables|/Game/Speedup/Blueprints/BP_LoginGameMode.BP_LoginGameMode_C|SetSignedIn _asbp_login_game_mode true))
  (return _output_get))

(fn GetSignedin
  (bind _asbp_login_game_mode (Utilities|Casting|CastToBP_LoginGameMode (Game|GetGameMode)))
  (return (Variables|/Game/Speedup/Blueprints/BP_LoginGameMode.BP_LoginGameMode_C|GetSignedIn _asbp_login_game_mode)))