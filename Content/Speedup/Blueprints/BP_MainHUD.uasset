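; Main HUD for an NFT-based app, managing wallet, statistics, active NFT, item, market and secondary screens.
; BeginPlay creates the screen widgets once and displays the wallet.
; Move functions switch screens by clearing widgets and re-adding the cached one, with main tabs also highlighting their tab bar icon.
; Item, slot, level-up, mint and profile calls mostly forward to Mouse_GameMode, cached in the Construction Script, or to child widgets.
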(event EventBeginPlay
  (Utilities|FlowControl|Sequence
    (:then_0
      (bind _returnvalue (Game|ConstructObjectfromClass (Game|GetPlayerController 0) "/Game/Speedup/Widgets/WalletSPDWidget_BP.WalletSPDWidget_BP_C"))
      (bind _output_get (Variables|Widgets|SetWalletDKSWidget _returnvalue))
      (UserInterface|Viewport|AddtoViewport _output_get 0))
    (:then_1
      (bind _returnvalue_2 (Game|ConstructObjectfromClass (Game|GetPlayerController 0) "/Game/Speedup/Widgets/StatisticsWidged_BP.StatisticsWidged_BP_C"))
      (Variables|Widgets|SetStatisticsWidged _returnvalue_2))
    (:then_2
      (bind _returnvalue_3 (Game|ConstructObjectfromClass (Game|GetPlayerController 0) "/Game/Speedup/Widgets/ActiveNFTsWidget_BP.ActiveNFTsWidget_BP_C"))
      (Variables|Widgets|SetActiveNFTsWidget _returnvalue_3))
    (:then_3
      (bind _returnvalue_4 (Game|ConstructObjectfromClass (Game|GetPlayerController 0) "/Game/Speedup/Widgets/ItemsWidget_BP.ItemsWidget_BP_C"))
      (Variables|Widgets|SetItemsWidget _returnvalue_4))
    (:then_4
      (bind _returnvalue_5 (Game|ConstructObjectfromClass (Game|GetPlayerController 0) "/Game/Speedup/Widgets/GeneralWidget_BP.GeneralWidget_BP_C"))
      (Variables|Widgets|SetGeneralWidget _returnvalue_5))
    (:then_5
      (bind _returnvalue_6 (Game|ConstructObjectfromClass (Game|GetPlayerController 0) "/Game/Speedup/Widgets/ChooseNFTWidget_BP.ChooseNFTWidget_BP_C"))
      (Variables|Widgets|SetChooseNFTWidget _returnvalue_6))
    (:then_6
      (bind _returnvalue_7 (Game|ConstructObjectfromClass (Game|GetPlayerController 0) "/Game/Speedup/Widgets/MarketWidget_BP.MarketWidget_BP_C"))
      (Variables|Widgets|SetMarket _returnvalue_7))
    (:then_7
      (bind _returnvalue_8 (Game|ConstructObjectfromClass (Game|GetPlayerController 0) "/Game/Speedup/Widgets/ChangePasswordWidget_BP.ChangePasswordWidget_BP_C"))
      (Variables|Default|SetChangePass _returnvalue_8))
    (:then_8
      (bind _returnvalue_9 (Game|ConstructObjectfromClass (Game|GetPlayerController 0) "/Game/Speedup/Widgets/CongratulationsWidget_BP.CongratulationsWidget_BP_C"))
      (Variables|Default|SetCongratulations _returnvalue_9))
    (:then_9
      (bind _returnvalue_10 (Game|ConstructObjectfromClass (Game|GetPlayerController 0) "/Game/Speedup/Widgets/DetailedCurrentItemWidget_BP.DetailedCurrentItemWidget_BP_C"))
      (Variables|Widgets|SetDetailedInfoWidget _returnvalue_10))
    (:then_10
      (bind _returnvalue_11 (Game|ConstructObjectfromClass (Game|GetPlayerController 0) "/Game/Speedup/Widgets/SuccessWidget_BP1.SuccessWidget_BP1_C"))
      (Variables|Default|SetWidgetMintSuccess _returnvalue_11))))

(event Collision|EventActorBeginOverlap
  (params (OtherActor :type Actor%20Object%20Reference)))

(event EventTick
  (params (DeltaSeconds :type Float%20%28single-precision%29)))

(fn ConstructionScript
  (bind _asmouse_game_mode (Utilities|Casting|CastToMouse_GameMode (Game|GetGameMode)))
  (Variables|GameMode|SetAs%20Mouse%20Game%20Mode _asmouse_game_mode)
  (Variables|Default|SetHTTPAPI (Variables|/Game/Speedup/Blueprints/Mouse_GameMode.Mouse_GameMode_C|GetHTTPAPI _asmouse_game_mode)))

(fn GetAllItems
  (Default|RequestGetAllNFT (Variables|GameMode|GetAs%20Mouse%20Game%20Mode)))

(fn ActiveItem
  (params (ItemID :type Integer) (Slot_N :type Integer))
  (Default|ActivateNFTSlot (Variables|GameMode|GetAs%20Mouse%20Game%20Mode) ItemID Slot_N))

(fn GetUserInfo)

(fn DeactiveItem
  (params (SlotID :type Integer) (ItemID :type Integer))
  (Default|DeactivateNFTSlot (Variables|GameMode|GetAs%20Mouse%20Game%20Mode) SlotID ItemID))

(fn ShowActiveNFTWidget
  (UserInterface|Viewport|AddtoViewport (Variables|Widgets|GetActiveNFTsWidget) 0))

(fn ShowChooseNFT
  (UserInterface|Viewport|AddtoViewport (Variables|Widgets|GetChooseNFTWidget) 0)
  (bind _asmouse_game_mode (Utilities|Casting|CastToMouse_GameMode (Game|GetGameMode)))
  (Default|SetChooseActive _asmouse_game_mode (Variables|Default|GetChoose%20Active)))

(fn HideChooseNFTWidget
  (Widget|RemovefromParent (Variables|Widgets|GetChooseNFTWidget)))

(fn MoveWalletWidget
  (bind _walletdkswidget (Variables|Widgets|GetWalletDKSWidget))
  (if (not (UserInterface|Viewport|IsinViewport (Variables|Widgets|GetWalletDKSWidget)))
    (Viewport|RemoveAllWidgets)
    (UserInterface|Viewport|AddtoViewport _walletdkswidget 0)
    (Default|ActiveIcon (Variables|/Game/Speedup/Widgets/WalletSPDWidget_BP.WalletSPDWidget_BP_C|GetBP_TabBarWidget _walletdkswidget))))

(fn MoveStatisticsWidget
  (bind _statisticswidged (Variables|Widgets|GetStatisticsWidged))
  (if (not (UserInterface|Viewport|IsinViewport (Variables|Widgets|GetStatisticsWidged)))
    (Viewport|RemoveAllWidgets)
    (UserInterface|Viewport|AddtoViewport _statisticswidged 0)
    (Default|ActiveIcon (Variables|/Game/Speedup/Widgets/StatisticsWidged_BP.StatisticsWidged_BP_C|GetBP_TabBarWidget _statisticswidged) 1)))

(fn MoveActiveNFTWidget
  (bind _activenftswidget (Variables|Widgets|GetActiveNFTsWidget))
  (if (not (UserInterface|Viewport|IsinViewport (Variables|Widgets|GetActiveNFTsWidget)))
    (Viewport|RemoveAllWidgets)
    (UserInterface|Viewport|AddtoViewport _activenftswidget 0)
    (Default|ActiveIcon (Variables|/Game/Speedup/Widgets/ActiveNFTsWidget_BP.ActiveNFTsWidget_BP_C|GetBP_TabBarWidget _activenftswidget) 2)))

(fn MoveItemsWidget
  (bind _itemswidget (Variables|Widgets|GetItemsWidget))
  (if (not (UserInterface|Viewport|IsinViewport (Variables|Widgets|GetItemsWidget)))
    (Viewport|RemoveAllWidgets)
    (UserInterface|Viewport|AddtoViewport _itemswidget 0)
    (Default|ActiveIcon (Variables|/Game/Speedup/Widgets/ItemsWidget_BP.ItemsWidget_BP_C|GetBP_TabBarWidget _itemswidget) 3)))

(fn MoveMarketWidget
  (bind _market (Variables|Widgets|GetMarket))
  (if (not (UserInterface|Viewport|IsinViewport (Variables|Widgets|GetMarket)))
    (Viewport|RemoveAllWidgets)
    (UserInterface|Viewport|AddtoViewport _market 0)
    (Default|ActiveIcon (Variables|/Game/Speedup/Widgets/MarketWidget_BP.MarketWidget_BP_C|GetBP_TabBarWidget _market) 4)))

(fn MovetoChangePassword
  (Viewport|RemoveAllWidgets)
  (UserInterface|Viewport|AddtoViewport (Variables|Default|GetChangePass) 0))

(fn MoveGeneralWidjet
  (Viewport|RemoveAllWidgets)
  (UserInterface|Viewport|AddtoViewport (Variables|Widgets|GetGeneralWidget) 0))

(fn HaveFreeSlots
  (bind _newparam (Default|HaveFreeSlots (Variables|GameMode|GetAs%20Mouse%20Game%20Mode)))
  (return _newparam))

(fn GetIteminSlot
  (params (SlotID :type Integer))
  (bind (_returnvalue _isempty _is_unlock) (Default|GetIteminSlot (Variables|GameMode|GetAs%20Mouse%20Game%20Mode) SlotID))
  (return _returnvalue _isempty _is_unlock))

(fn RefreshActiveItemsRequest
  (Default|Refresh (Variables|Widgets|GetActiveNFTsWidget)))

(fn RefreshProfileRequest
  (Default|RequestProfile (Variables|GameMode|GetAs%20Mouse%20Game%20Mode)))

(fn RemoveMainHUDWidgets
  (Utilities|FlowControl|Sequence
    (:then_0
      (Utilities|Remove (Variables|Widgets|GetWalletDKSWidget)))
    (:then_1
      (Utilities|Remove (Variables|Widgets|GetStatisticsWidged)))
    (:then_2
      (Utilities|Remove (Variables|Widgets|GetActiveNFTsWidget)))
    (:then_3
      (Utilities|Remove (Variables|Widgets|GetItemsWidget)))
    (:then_4
      (Utilities|Remove (Variables|Widgets|GetChooseNFTWidget)))
    (:then_5
      (Utilities|Remove (Variables|Widgets|GetGeneralWidget)))
    (:then_6
      (Utilities|Remove (Variables|Widgets|GetMarketWidget)))))

(fn MovetoDetailedInfo
  (params (Item :type Item%20Object%20Reference))
  (bind _detailedinfowidget (Variables|Widgets|GetDetailedInfoWidget))
  (Viewport|RemoveAllWidgets)
  (UserInterface|Viewport|AddtoViewport _detailedinfowidget 0)
  (Default|Init _detailedinfowidget Item)
  (Default|FillLevelProgressBar _detailedinfowidget Item)
  (Default|FillTerms _detailedinfowidget Item)
  (Default|FillLevelLeft _detailedinfowidget Item))

(fn MovetoMintSucces
  (Viewport|RemoveAllWidgets)
  (UserInterface|Viewport|AddtoViewport (Variables|Default|GetWidgetMintSuccess) 0))

(fn MovetoCongratuations
  (Viewport|RemoveAllWidgets)
  (UserInterface|Viewport|AddtoViewport (Variables|Default|GetCongratulations) 0))

(fn OpenDetail
  (params (Item :type Item%20Object%20Reference))
  (Default|DetailedOpen1 (Variables|Widgets|GetItemsWidget) Item))

(fn LvlUpRequest
  (params (id :type Integer))
  (Default|LevelUpRequest (Variables|GameMode|GetAs%20Mouse%20Game%20Mode) id))

(fn GetItem
  (params (id :type Integer))
  (bind _item_ (Default|GetItem (Variables|GameMode|GetAs%20Mouse%20Game%20Mode) id))
  (return _item_))

(fn CheckLvlUpPossible
  (params (item :type Item%20Object%20Reference))
  (bind _nextlevelenabled (Default|CheckLevelUpAbillity (Variables|Widgets|GetDetailedInfoWidget) item))
  (return _nextlevelenabled))

(fn NFTmint
  (params (id :type Integer))
  (Default|MintItem (Variables|GameMode|GetAs%20Mouse%20Game%20Mode) id))