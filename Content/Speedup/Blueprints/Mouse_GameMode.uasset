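; Game mode for SpeedUp that acts as a facade for NFT, geo path tracking and wallet features.
; It initializes HTTPAPI on BeginPlay, forwards NFT list and slot requests to it, and passes path start/stop calls to BPSpeedUpGeoSystem.
; It also stores NFT selection and icon state, and reads wallet address and balance from the game instance.
; Slot deactivation always sends 1, and ChecActivSlots only copies values into locals.
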(event EventBeginPlay
  (Class|HTTPAPIComponent|InitComponent (Variables|Default|GetHTTPAPI)))

(event EventTick
  (params (DeltaSeconds :type Float%20%28single-precision%29)))

(fn ConstructionScript)

(fn SetChoosenNFT
  (params (NewNFT :type Integer))
  (Variables|Default|SetChoosenNFT NewNFT))

(fn GetChoosenNFT
  (return (Variables|Default|GetChoosenNFT)))

(fn SetTabIconVis
  (params (Icon :type Integer))
  (Variables|Default|SetIconVisibility Icon))

(fn GetTabIconVis
  (return (Variables|Default|GetIconVisibility)))

(fn RequestGetAllNFT
  (bind _httpapi (Variables|Default|GetHTTPAPI))
  (Class|HTTPAPIComponent|NFTreceiptRequest _httpapi (Variables|/Script/speedup.HTTPAPIComponent|GetClientTocken _httpapi)))

(fn StartPath
  (params (PuthN :type Integer))
  (Class|SpeedupGeoDataSystem|StartTrackPath (Variables|Default|GetBP_SpeedUp_GeoSystem) PuthN))

(fn StopPath
  (params (PuthN :type Integer))
  (Class|SpeedupGeoDataSystem|StopTrackPath (Variables|Default|GetBP_SpeedUp_GeoSystem) PuthN))

(fn ActivateNFTSlot
  (params (ActivNFTId :type Integer) (SlotID :type Integer))
  (Class|HTTPAPIComponent|NFTactivationRequest (Variables|Default|GetHTTPAPI) ActivNFTId))

(fn DeactivateNFTSlot
  (Class|HTTPAPIComponent|NFTdeactivationRequest (Variables|Default|GetHTTPAPI) 1))

(fn ChecActivSlots
  (bind _httpapi (Variables|Default|GetHTTPAPI))
  (LocalVariables|SetErr (Variables|/Script/speedup.HTTPAPIComponent|GetErrorID _httpapi))
  (LocalVariables|SetMess (Variables|/Script/speedup.HTTPAPIComponent|GetMessage _httpapi))
  (LocalVariables|SetNewLocalVar_1 (Variables|/Script/speedup.HTTPAPIComponent|GetPathID _httpapi))
  (for _array_element (Variables|/Script/speedup.ItemManager|GetItemsSlot (Variables|Default|GetNFTItemManager))
    (LocalVariables|SetNewLocalVar_0 (.ItemID (Utilities|Struct|BreakItemSlot _array_element)))
    (LocalVariables|SetPath (.PathForItem (Utilities|Struct|BreakItemSlot _array_element)))))

(fn SetChooseActive
  (params (bool :type Boolean))
  (Variables|Default|SetChooseActive bool))

(fn GetChooseActive
  (return (Variables|Default|GetChooseActive)))

(fn GetWalletAddress
  (bind _asspeed_up_game_instance (Utilities|Casting|CastToSpeedUpGameInstance (Game|GetGameInstance)))
  (return (.dks_wallet (.balance (Variables|/Script/speedup.SpeedUpGameInstance|GetUserInfo _asspeed_up_game_instance)))))

(fn GetBalance
  (bind _asspeed_up_game_instance (Utilities|Casting|CastToSpeedUpGameInstance (Game|GetGameInstance)))
  (return (.dks_balance (.balance (Variables|/Script/speedup.SpeedUpGameInstance|GetUserInfo _asspeed_up_game_instance)))))