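; Login HUD that manages the account screens for sign-up, sign-in, code entry and password recovery.
; BeginPlay pre-constructs the widgets and shows sign-in; MoveTo functions switch screens by clearing widgets and adding the target, some with a transition sound.
; Recovery and Google auth requests go to the HTTP object from LoginGameModeBase, while Logout uses Mouse_GameMode's.
; Login, password and a save flag persist in the "Login" save slot.
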(event EventBeginPlay
  (Utilities|FlowControl|Sequence
    (:then_0
      (bind _returnvalue (Game|ConstructObjectfromClass (Game|GetPlayerController 0) "/Game/Speedup/Widgets/SignUpWidget_BP.SignUpWidget_BP_C"))
      (Variables|Default|SetSignUpWidget _returnvalue))
    (:then_1
      (bind _returnvalue_2 (Game|ConstructObjectfromClass (Game|GetPlayerController 0) "/Game/Speedup/Widgets/SignUpEnterWidget_BP.SignUpEnterWidget_BP_C"))
      (Variables|Default|SetSignUpEnterWidget _returnvalue_2))
    (:then_2
      (bind _returnvalue_3 (Game|ConstructObjectfromClass (Game|GetPlayerController 0) "/Game/Speedup/Widgets/SignInWidget_BP1.SignInWidget_BP1_C"))
      (bind _output_get (Variables|Default|SetSignInWidget _returnvalue_3))
      (UserInterface|Viewport|AddtoViewport _output_get 0))
    (:then_3
      (bind _returnvalue_4 (Game|ConstructObjectfromClass (Game|GetPlayerController 0) "/Game/Speedup/Widgets/SignInEnterWidget_BP.SignInEnterWidget_BP_C"))
      (Variables|Default|SetSignInEnterWidget _returnvalue_4))
    (:then_4
      (bind _returnvalue_5 (Game|ConstructObjectfromClass (Game|GetPlayerController 0) "/Game/Speedup/Widgets/EnterCodeWidget_BP.EnterCodeWidget_BP_C"))
      (Variables|Default|SetEnterCodeWidget _returnvalue_5))
    (:then_5
      (bind _returnvalue_6 (Game|ConstructObjectfromClass (Game|GetPlayerController 0) "/Game/Speedup/Widgets/ForgotPasswordWidget_BP.ForgotPasswordWidget_BP_C"))
      (Variables|Default|SetForgotPasswordWidget _returnvalue_6))
    (:then_6
      (bind _returnvalue_7 (Game|ConstructObjectfromClass (Game|GetPlayerController 0) "/Game/Speedup/Widgets/EnterNewPasswordWidget_BP.EnterNewPasswordWidget_BP_C"))
      (Variables|Default|SetEnterNewPassword _returnvalue_7))
    (:then_7
      (bind _returnvalue_8 (Game|ConstructObjectfromClass (Game|GetPlayerController 0) "/Game/Speedup/Widgets/CongratulationsWidget_BP.CongratulationsWidget_BP_C"))
      (Variables|Default|SetCongratulationsWidgetBP _returnvalue_8))
    (:then_8
      (bind _returnvalue_9 (Game|ConstructObjectfromClass (Game|GetPlayerController 0) "/Game/Speedup/Widgets/SignCongratulationsWidget_BP1.SignCongratulationsWidget_BP1_C"))
      (Variables|Default|SetSignUpSuccess _returnvalue_9))
    (:then_9
      (bind _returnvalue_10 (Game|ConstructObjectfromClass (Game|GetPlayerController 0) "/Game/Speedup/Widgets/GeneralWidget_BP.GeneralWidget_BP_C"))
      (Variables|Default|SetgeneralW _returnvalue_10))))

(event Collision|EventActorBeginOverlap
  (params (OtherActor :type Actor%20Object%20Reference)))

(event EventTick
  (params (DeltaSeconds :type Float%20%28single-precision%29)))

(fn ConstructionScript
  (bind _aslogin_game_mode_base (Utilities|Casting|CastToLoginGameModeBase (Game|GetGameMode)))
  (Variables|Default|SetHTTPAPI (Variables|/Script/speedup.LoginGameModeBase|GetHTTP _aslogin_game_mode_base)))

(fn ShowSignUpWidget
  (UserInterface|Viewport|AddtoViewport (Variables|Default|GetSignUpWidget) 0))

(fn HideSignUpWidget
  (Widget|RemovefromParent (Variables|Default|GetSignUpWidget)))

(fn ShowSignUpEnterWidget
  (UserInterface|Viewport|AddtoViewport (Variables|Default|GetSignUpEnterWidget) 0))

(fn HideSignUpEnterWidget
  (Widget|RemovefromParent (Variables|Default|GetSignUpEnterWidget)))

(fn ShowSigninWidget
  (UserInterface|Viewport|AddtoViewport (Variables|Default|GetSignInWidget) 0))

(fn HideSigninWidget
  (Widget|RemovefromParent (Variables|Default|GetSignInWidget)))

(fn ShowSigninEnterWidget
  (UserInterface|Viewport|AddtoViewport (Variables|Default|GetSignInEnterWidget) 0))

(fn HideSigninEnterWidget
  (Widget|RemovefromParent (Variables|Default|GetSignInEnterWidget)))

(fn ShowEnterCodeWidget
  (UserInterface|Viewport|AddtoViewport (Variables|Default|GetEnterCodeWidget) 0))

(fn HideEnterCodeWidget
  (Widget|RemovefromParent (Variables|Default|GetEnterCodeWidget)))

(fn MovetoSignUpWidget
  (Viewport|RemoveAllWidgets)
  (UserInterface|Viewport|AddtoViewport (Variables|Default|GetSignUpWidget) 0)
  (CallFunction|PlaySoundNext))

(fn MovetoSignUpEnterWidget
  (CallFunction|RemoveAllWidjet)
  (UserInterface|Viewport|AddtoViewport (Variables|Default|GetSignUpEnterWidget) 0)
  (CallFunction|PlaySoundNext))

(fn MovetoSigninWidget
  (Viewport|RemoveAllWidgets)
  (UserInterface|Viewport|AddtoViewport (Variables|Default|GetSignInWidget) 0)
  (CallFunction|PlaySoundNext))

(fn MovetoSigninEnterWidget
  (Viewport|RemoveAllWidgets)
  (UserInterface|Viewport|AddtoViewport (Variables|Default|GetSignInEnterWidget) 0)
  (CallFunction|PlaySoundNext))

(fn MovetoEnterCodeWidget
  (Viewport|RemoveAllWidgets)
  (UserInterface|Viewport|AddtoViewport (Variables|Default|GetEnterCodeWidget) 0))

(fn MovetoForgotPasswordWidget
  (CallFunction|RemoveAllWidjet)
  (UserInterface|Viewport|AddtoViewport (Variables|Default|GetForgotPasswordWidget) 0))

(fn MovetoEnterNewPasswordWidget
  (CallFunction|RemoveAllWidjet)
  (UserInterface|Viewport|AddtoViewport (Variables|Default|GetEnterNewPassword) 0))

(fn RemoveAllWidjet
  (Utilities|FlowControl|Sequence
    (:then_0
      (Utilities|CheckandRemove (Variables|Default|GetSignUpEnterWidget)))
    (:then_1
      (Utilities|CheckandRemove (Variables|Default|GetSignUpEnterWidget)))
    (:then_2
      (Utilities|CheckandRemove (Variables|Default|GetSignInWidget)))
    (:then_3
      (Utilities|CheckandRemove (Variables|Default|GetSignInEnterWidget)))
    (:then_4
      (Utilities|CheckandRemove (Variables|Default|GetSignInEnterWidget)))
    (:then_5
      (Utilities|CheckandRemove (Variables|Default|GetForgotPasswordWidget)))
    (:then_6
      (Utilities|CheckandRemove (Variables|Default|GetEnterNewPassword)))))

(fn LaodLoginPassword
  (bind _returnvalue (SaveGame|LoadGamefromSlot "Login"))
  (bind _asbp_save_login_password (Utilities|Casting|CastToBP_SaveLoginPassword _returnvalue)
    (:then
      (return (Variables|/Game/Speedup/Blueprints/BP_SaveLoginPassword.BP_SaveLoginPassword_C|GetIsSave _asbp_save_login_password) (Variables|/Game/Speedup/Blueprints/BP_SaveLoginPassword.BP_SaveLoginPassword_C|GetLogin _asbp_save_login_password) (Variables|/Game/Speedup/Blueprints/BP_SaveLoginPassword.BP_SaveLoginPassword_C|GetPassword _asbp_save_login_password)))
    (:CastFailed
      (return true "" ""))))

(fn SaveLoginPassword
  (params (Login :type String) (Password :type String) (IsSave :type Boolean))
  (bind _returnvalue (SaveGame|CreateSaveGameObject "/Game/Speedup/Blueprints/BP_SaveLoginPassword.BP_SaveLoginPassword_C"))
  (bind _output_get (LocalVariables|SetUresInfo _returnvalue))
  (Variables|/Game/Speedup/Blueprints/BP_SaveLoginPassword.BP_SaveLoginPassword_C|SetLogin _output_get Login)
  (Variables|/Game/Speedup/Blueprints/BP_SaveLoginPassword.BP_SaveLoginPassword_C|SetPassword _output_get Password)
  (Variables|/Game/Speedup/Blueprints/BP_SaveLoginPassword.BP_SaveLoginPassword_C|SetIsSave _output_get IsSave)
  (SaveGame|SaveGametoSlot _output_get "Login"))

(fn MovetoChangePasswordWidget
  (CallFunction|RemoveAllWidjet)
  (UserInterface|Viewport|AddtoViewport (Variables|Default|GetChangePasswordWidget) 0))

(fn MovetoCongratulationsWidget
  (CallFunction|RemoveAllWidjet)
  (UserInterface|Viewport|AddtoViewport (Variables|Default|GetCongratulationsWidgetBP) 0))

(fn SendCodeRecovery
  (params (email :type String))
  (Class|HTTPAPIComponent|SendRecoveryCode (Variables|Default|GetHTTPAPI) email))

(fn SuccessorNot
  (bind _aslogin_game_mode_base (Utilities|Casting|CastToLoginGameModeBase (Game|GetGameMode)))
  (bind _output_get (Variables|Default|SetHTTPAPI (Variables|/Script/speedup.LoginGameModeBase|GetHTTP _aslogin_game_mode_base)))
  (return (Variables|/Script/speedup.HTTPAPIComponent|GetbSuccess _output_get)))

(fn RepairPassword
  (params (code :type String) (passwordNew :type String) (email :type String))
  (Class|HTTPAPIComponent|RepairPassword (Variables|Default|GetHTTPAPI) passwordNew code email))

(fn Logout
  (bind _asmouse_game_mode (Utilities|Casting|CastToMouse_GameMode (Game|GetGameMode)))
  (Class|HTTPAPIComponent|LogoutRequest (Variables|/Game/Speedup/Blueprints/Mouse_GameMode.Mouse_GameMode_C|GetHTTPAPI _asmouse_game_mode) (Variables|/Script/speedup.HTTPAPIComponent|GetData (Variables|/Game/Speedup/Blueprints/Mouse_GameMode.Mouse_GameMode_C|GetHTTPAPI _asmouse_game_mode))))

(fn PlaySoundNext
  (Audio|PlaySound2D "/Game/Speedup/Sounds/S_mixkit-video-game-mystery-alert-234.S_mixkit-video-game-mystery-alert-234" 1.0 1.0 0.0 0 0))

(fn PlaySoundError
  (Audio|PlaySound2D "/Game/Speedup/Sounds/S_mixkit-digital-quick-tone-2866.S_mixkit-digital-quick-tone-2866" 1.0 1.0 0.0 0 0))

(fn MovetoSignSuccess
  (Viewport|RemoveAllWidgets)
  (UserInterface|Viewport|AddtoViewport (Variables|Default|GetSignUpSuccess) 0))

(fn GoogleAuthRequest
  (Class|HTTPAPIComponent|GoogleAuth (Variables|Default|GetHTTPAPI)))